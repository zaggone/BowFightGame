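; BP_BFGBaseCharacter is a player character Blueprint that records movement and jump input signals as simple state variables.
; On BeginPlay it binds handlers to the moving-along, moving-across and jump event dispatchers.
; The movement handlers store the incoming axis amounts, while the jump handler raises IsJump and clears it after a short fixed Delay, independent of landing.
; Tick and the construction script are empty.
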(event `self.ReceiveBeginPlay`
  (add `self.OnMovingAlong` (delegate `OnMovingAlong_Event_0`))
  (add `self.OnMovingAcross` (delegate `OnMovingAcross_Event_0`))
  (add `self.OnJump` (delegate `OnJump_Event_0`)))

(event `OnMovingAlong_Event_0` :!signature `self.OnMovingAlong`
  (params (Amount :type "Float (double-precision)"))
  (set `self.MoveAlongAmount` Amount))

(event `OnJump_Event_0`
  (set `self.IsJump` true)
  (`KismetSystemLibrary.Delay` 0.5)
  (set `self.IsJump` false))

(event `OnMovingAcross_Event_0` :!signature `self.OnMovingAcross`
  (params (Amount :type "Float (double-precision)"))
  (set `self.MoveAcrossAmount` Amount))

(event `self.ReceiveTick`
  (params (DeltaSeconds :type "Float (single-precision)")))

(fn `UserConstructionScript`)